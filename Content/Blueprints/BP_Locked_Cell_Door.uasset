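; Locked cell door that the player unlocks with a key and swings open with E.
; Box overlap enables input and sets HasKey if the character holds at least one key.
; E without a key shakes the lock; with one, it unlocks, sets KeyCount to -1 and destroys the lock.
; Once unlocked, E plays yaw timelines chosen by the Front trigger, with a delayed second timeline after each opening one.
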(event `self.Front.OnComponentBeginOverlap`
  (params (OverlappedComponent :type "PrimitiveComponent Object Reference") (OtherActor :type "Actor Object Reference") (OtherComp :type "PrimitiveComponent Object Reference") (OtherBodyIndex :type Integer) (bFromSweep :type Boolean) (SweepResult :type "HitResult Structure (by ref)"))
  (set `self.AtFrontDoor` true))

(event `self.Front.OnComponentEndOverlap`
  (params (OverlappedComponent :type "PrimitiveComponent Object Reference") (OtherActor :type "Actor Object Reference") (OtherComp :type "PrimitiveComponent Object Reference") (OtherBodyIndex :type Integer))
  (set `self.AtFrontDoor` false))

(event `self.Box.OnComponentBeginOverlap`
  (params (OverlappedComponent :type "PrimitiveComponent Object Reference") (OtherActor :type "Actor Object Reference") (OtherComp :type "PrimitiveComponent Object Reference") (OtherBodyIndex :type Integer) (bFromSweep :type Boolean) (SweepResult :type "HitResult Structure (by ref)"))
  (`self.EnableInput` (`GameplayStatics.GetPlayerController` 0))
  (if (not (`self.HasKey`))
    (bind _ascapstone_2077character (cast `Capstone2077Character` (`GameplayStatics.GetPlayerCharacter` 0)))
    (bind _returnvalue (`Capstone2077Character.GetKeyCount` _ascapstone_2077character))
    (`/Engine/EditorBlueprintResources/StandardMacros.CompareInt` _returnvalue 1
      (:`>`
        _)
      (:`==`
        _))
    (set `self.HasKey` true)))

(event `self.Box.OnComponentEndOverlap`
  (params (OverlappedComponent :type "PrimitiveComponent Object Reference") (OtherActor :type "Actor Object Reference") (OtherComp :type "PrimitiveComponent Object Reference") (OtherBodyIndex :type Integer))
  (`self.DisableInput` (`GameplayStatics.GetPlayerController` 0)))

(event `Key|E`
  (params (Key :type "Key Structure"))
  (:`Pressed`
    (if (`self.IsUnlocked`)
      (if (`self.AtFrontDoor`)
        (bind (_direction _dooropen) (`Timeline|Timeline_0` :!via `PlayFromStart`)
          (:`Update`
            (`SceneComponent.K2_SetRelativeRotation` (`self.SM_Cell_Door`) (`KismetMathLibrary.MakeRotator` 0.0 0.0 _dooropen) false false)
            (`KismetSystemLibrary.Delay` 2.0)
            (bind (_direction_2 _dooropen_2) (`Timeline|Timeline_1` :!via `PlayFromStart`)
              (:`Update`
                (`SceneComponent.K2_SetRelativeRotation` (`self.SM_Cell_Door`) (`KismetMathLibrary.MakeRotator` 0.0 0.0 _dooropen_2) false false)))))
        (else
          (bind (_direction_3 _dooropen_3) (`Timeline|Timeline_2` :!via `PlayFromStart`)
            (:`Update`
              (`SceneComponent.K2_SetRelativeRotation` (`self.SM_Cell_Door`) (`KismetMathLibrary.MakeRotator` 0.0 0.0 _dooropen_3) false false)
              (`KismetSystemLibrary.Delay` 2.0)
              (bind (_direction_4 _dooropen_4) (`Timeline|Timeline_3` :!via `PlayFromStart`)
                (:`Update`
                  (`SceneComponent.K2_SetRelativeRotation` (`self.SM_Cell_Door`) (`KismetMathLibrary.MakeRotator` 0.0 0.0 _dooropen_4) false false)))))))
      (elif (`self.HasKey`)
        (set `self.IsUnlocked` true)
        (bind _ascapstone_2077character (cast `Capstone2077Character` (`GameplayStatics.GetPlayerCharacter` 0)))
        (set `Capstone2077Character.KeyCount` -1 _ascapstone_2077character)
        (`ActorComponent.K2_DestroyComponent` (`self.SM_Lock_Closed`))
        (else
          (bind (_direction_5 _shakelock) (`Timeline|Timeline_4` :!via `PlayFromStart`)
            (:`Update`
              (`SceneComponent.K2_SetRelativeRotation` (`self.SM_Lock_Closed`) (`KismetMathLibrary.MakeRotator` 90.0 _shakelock -80.0) false false)
              (`KismetSystemLibrary.Delay` 2.0)
              (bind (_direction_6 _shakelock_2) (`Timeline|Timeline_5` :!via `PlayFromStart`)))))))))

(fn `UserConstructionScript`)