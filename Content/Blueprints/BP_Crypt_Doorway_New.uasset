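; Crypt doorway Blueprint with two large doors that rotate when the player presses E.
; The Box overlap toggles player input, while Box1 sets AtFrontDoor to choose which timelines drive each door's yaw, apparently so the swing depends on the side.
; Two E handlers animate the right and left doors separately, each chaining a second timeline, likely the close, through a two-second Delay wired from Update rather than Finished.
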(event `self.Box1.OnComponentBeginOverlap`
  (params (OverlappedComponent :type "PrimitiveComponent Object Reference") (OtherActor :type "Actor Object Reference") (OtherComp :type "PrimitiveComponent Object Reference") (OtherBodyIndex :type Integer) (bFromSweep :type Boolean) (SweepResult :type "HitResult Structure (by ref)"))
  (set `self.AtFrontDoor` true))

(event `self.Box1.OnComponentEndOverlap`
  (params (OverlappedComponent :type "PrimitiveComponent Object Reference") (OtherActor :type "Actor Object Reference") (OtherComp :type "PrimitiveComponent Object Reference") (OtherBodyIndex :type Integer))
  (set `self.AtFrontDoor` false))

(event `self.Box.OnComponentBeginOverlap`
  (params (OverlappedComponent :type "PrimitiveComponent Object Reference") (OtherActor :type "Actor Object Reference") (OtherComp :type "PrimitiveComponent Object Reference") (OtherBodyIndex :type Integer) (bFromSweep :type Boolean) (SweepResult :type "HitResult Structure (by ref)"))
  (`self.EnableInput` (`GameplayStatics.GetPlayerController` 0)))

(event `self.Box.OnComponentEndOverlap`
  (params (OverlappedComponent :type "PrimitiveComponent Object Reference") (OtherActor :type "Actor Object Reference") (OtherComp :type "PrimitiveComponent Object Reference") (OtherBodyIndex :type Integer))
  (`self.DisableInput` (`GameplayStatics.GetPlayerController` 0)))

(event `Key|E`
  (params (Key :type "Key Structure"))
  (:`Pressed`
    (if (`self.AtFrontDoor`)
      (bind (_direction _dooropen) (`Timeline|Timeline_3` :!via `PlayFromStart`)
        (:`Update`
          (`SceneComponent.K2_SetRelativeRotation` (`self.SM_DoorWay_Large_Door_Right`) (`KismetMathLibrary.MakeRotator` 0.0 0.0 _dooropen) false false)
          (`KismetSystemLibrary.Delay` 2.0)
          (bind (_direction_2 _dooropen_2) (`Timeline|Timeline_4` :!via `PlayFromStart`)
            (:`Update`
              (`SceneComponent.K2_SetRelativeRotation` (`self.SM_DoorWay_Large_Door_Right`) (`KismetMathLibrary.MakeRotator` 0.0 0.0 _dooropen_2) false false)))))
      (else
        (bind (_direction_3 _dooropen_3) (`Timeline|DoorRotate` :!via `PlayFromStart`)
          (:`Update`
            (`SceneComponent.K2_SetRelativeRotation` (`self.SM_DoorWay_Large_Door_Right`) (`KismetMathLibrary.MakeRotator` 0.0 0.0 _dooropen_3) false false)
            (`KismetSystemLibrary.Delay` 2.0)
            (bind (_direction_4 _dooropen_4) (`Timeline|Timeline_1` :!via `PlayFromStart`)
              (:`Update`
                (`SceneComponent.K2_SetRelativeRotation` (`self.SM_DoorWay_Large_Door_Right`) (`KismetMathLibrary.MakeRotator` 0.0 0.0 _dooropen_4) false false)))))))))

(event `Key|E`
  (params (Key :type "Key Structure"))
  (:`Pressed`
    (if (`self.AtFrontDoor`)
      (bind (_direction _dooropen) (`Timeline|Timeline_5` :!via `PlayFromStart`)
        (:`Update`
          (`SceneComponent.K2_SetRelativeRotation` (`self.SM_DoorWay_Large_Door_Left`) (`KismetMathLibrary.MakeRotator` 0.0 0.0 _dooropen) false false)
          (`KismetSystemLibrary.Delay` 2.0)
          (bind (_direction_2 _dooropen_2) (`Timeline|Timeline_6` :!via `PlayFromStart`)
            (:`Update`
              (`SceneComponent.K2_SetRelativeRotation` (`self.SM_DoorWay_Large_Door_Left`) (`KismetMathLibrary.MakeRotator` 0.0 0.0 _dooropen_2) false false)))))
      (else
        (bind (_direction_3 _dooropen_3) (`Timeline|Timeline_0` :!via `PlayFromStart`)
          (:`Update`
            (`SceneComponent.K2_SetRelativeRotation` (`self.SM_DoorWay_Large_Door_Left`) (`KismetMathLibrary.MakeRotator` 0.0 0.0 _dooropen_3) false false)
            (`KismetSystemLibrary.Delay` 2.0)
            (bind (_direction_4 _dooropen_4) (`Timeline|Timeline_2` :!via `PlayFromStart`)
              (:`Update`
                (`SceneComponent.K2_SetRelativeRotation` (`self.SM_DoorWay_Large_Door_Left`) (`KismetMathLibrary.MakeRotator` 0.0 0.0 _dooropen_4) false false)))))))))

(fn `UserConstructionScript`)