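; Enemy shooter actor that turns toward the first-person player and fires projectiles whenever it sees them.
; PawnSensing's see-pawn event snaps the actor's rotation to face the character, then spawns a FirstPersonProjectile at the spawn-location component.
; The projectile's mesh receives a velocity-change impulse along the Cube's forward vector scaled by ShootForce.
; A SpawnProjectile flag with a delay acts as a fire-rate cooldown between shots.
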(event `self.PawnSensing.OnSeePawn`
  (params (Pawn :type "Pawn Object Reference"))
  (bind _asfirst_person_character (cast `/Game/FirstPersonCPP/Blueprints/FirstPersonCharacter` Pawn))
  (`|ExecutionSequence`
    (:`then_0`
      (`self.K2_SetActorRotation` (`KismetMathLibrary.FindLookAtRotation` (`self.K2_GetActorLocation`) (`self.K2_GetActorLocation` _asfirst_person_character))))
    (:`then_1`
      (if (`self.SpawnProjectile`)
        (bind _returnvalue (`|SpawnActorFromClass` "/Game/FirstPersonCPP/Blueprints/FirstPersonProjectile.FirstPersonProjectile_C" (`SceneComponent.K2_GetComponentToWorld` (`self.ProjectileSpawnLocation`)) "Undefined" "OverrideRootScale" null null))
        (`PrimitiveComponent.AddImpulse` (`/Game/FirstPersonCPP/Blueprints/FirstPersonProjectile.StaticMesh1` _returnvalue) (* (`SceneComponent.GetForwardVector` (`self.Cube`)) (`self.ShootForce`)) "None" true)
        (set `self.SpawnProjectile` false)
        (`KismetSystemLibrary.Delay` 1.5)
        (set `self.SpawnProjectile` true)))))

(fn `UserConstructionScript`)